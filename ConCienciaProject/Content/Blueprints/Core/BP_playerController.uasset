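; Player controller that sets up the game's UI on begin play and provides an event that opens the pause menu.
; It adds the HUD, matches the current level name to add that level's own widget (Quino, Mateo, Ana, Liu, Final Exam), then layers a difficulty chooser on top.
; The chooser is created early so its title can be set per level, except for Final Exam.
; The difficultyChosen event is an empty stub.
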(event `self.ReceiveBeginPlay`
  (bind _leveltitletext (`/Game/Blueprints/Widgets/UI_chooseDifficulty.levelTitleText` (`self.chooseDiff_UI_reference`)))
  ;[1 0.3859 0 0.5] begin play
  (`|ExecutionSequence`
    (:`then_0`
      (`self.EnableInput` (`GameplayStatics.GetPlayerController` 0)))
    (:`then_1`
      (bind _returnvalue (`|CreateWidget` "/Game/Blueprints/Widgets/UI_HUD.UI_HUD_C"))
      (`UserWidget.AddToViewport` _returnvalue 0)
      ;;[1 0 0.04507 0.5] create the choose difficulty but dont add it to viewport yet
      (bind _returnvalue_2 (`|CreateWidget` "/Game/Blueprints/Widgets/UI_chooseDifficulty.UI_chooseDifficulty_C"))
      (set `self.chooseDiff_UI_reference` _returnvalue_2))
    (:`then_2`
      ;;[1 0.5152 0 0.5] open ui depending on current level
      (`|ExecutionSequence`
        (:`then_0`
          (bind _returnvalue_3 (`GameplayStatics.GetCurrentLevelName` true))
          (switch `name` (`KismetStringLibrary.Conv_StringToName` _returnvalue_3)
            (:`LVL_quino`
              (bind _returnvalue_4 (`|CreateWidget` "/Game/Blueprints/Widgets/minigames/quino/UI_quino.UI_quino_C"))
              (`UserWidget.AddToViewport` _returnvalue_4 0)
              (`TextBlock.SetText` _leveltitletext "Quino's Level"))
            (:`LVL_mateo`
              (bind _returnvalue_5 (`|CreateWidget` "/Game/Blueprints/Widgets/minigames/mateo/UI_mateo.UI_mateo_C"))
              (`UserWidget.AddToViewport` _returnvalue_5 0)
              (`TextBlock.SetText` _leveltitletext "Mateo's Level"))
            (:`LVL_ana`
              (bind _returnvalue_6 (`|CreateWidget` "/Game/Blueprints/Widgets/minigames/ana/UI_ana.UI_ana_C"))
              (`UserWidget.AddToViewport` _returnvalue_6 0)
              (`TextBlock.SetText` _leveltitletext "Ana's Level"))
            (:`LVL_liu`
              (bind _returnvalue_7 (`|CreateWidget` "/Game/Blueprints/Widgets/minigames/liu/UI_liu.UI_liu_C"))
              (`UserWidget.AddToViewport` _returnvalue_7 0)
              (`TextBlock.SetText` _leveltitletext "Liu's Level"))
            (:`LVL_finalExam`
              (bind _returnvalue_8 (`|CreateWidget` "/Game/Blueprints/Widgets/minigames/finalExam/UI_finalExam.UI_finalExam_C"))
              (`UserWidget.AddToViewport` _returnvalue_8 0))))
        (:`then_1`
          (if true
            ;;;[1 0 0.01209 0.5] now you can add to viewport, on top of the other one
            (`UserWidget.AddToViewport` (`self.chooseDiff_UI_reference`) 0)))))))

(event `openPauseMenu`
  (bind _returnvalue (`|CreateWidget` "/Game/Blueprints/Widgets/UI_pauseMenu.UI_pauseMenu_C"))
  (`UserWidget.AddToViewport` _returnvalue 0))

(event `difficultyChosen`
  (params (difficultyIndex :type Integer)))

(fn `UserConstructionScript`)